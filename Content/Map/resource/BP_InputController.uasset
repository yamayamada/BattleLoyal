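; BP_InputController turns one player's gamepad input into discrete, player-tagged calls for buttons and stick flicks.
; BeginPlay caches the Player's controller and ID; GetPlayer can refill an invalid Player from MyGameInstance.
; Tick polls A, B, Start and both sticks, firing once per press via DoOnce, with hysteresis on stick axes.
; Start passes the controller instead of the player number, and positive stick X triggers the "Left" calls.
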(event `self.ReceiveBeginPlay`
  (bind _asplayer_controller (cast `PlayerController` (`Pawn.GetController` (`self.Player`))))
  (set `self.Controller` _asplayer_controller)
  (bind _returnvalue (`GameplayStatics.GetPlayerControllerID` _asplayer_controller))
  (set `self.PlayerNumber` _returnvalue))

(event `self.ReceiveTick`
  (params (DeltaSeconds :type "Float (single-precision)"))
  (bind _controller (`self.Controller`))
  (bind _returnvalue (`PlayerController.GetInputAnalogKeyState` _controller "Gamepad_LeftY"))
  (bind _returnvalue_2 (`PlayerController.GetInputAnalogKeyState` _controller "Gamepad_RightY"))
  (bind _returnvalue_3 (`PlayerController.GetInputAnalogKeyState` _controller "Gamepad_RightY"))
  (bind _returnvalue_4 (`PlayerController.GetInputAnalogKeyState` _controller "Gamepad_RightX"))
  (bind _returnvalue_5 (`PlayerController.GetInputAnalogKeyState` _controller "Gamepad_LeftX"))
  (bind _returnvalue_6 (`PlayerController.GetInputAnalogKeyState` _controller "Gamepad_LeftX"))
  (bind _returnvalue_7 (`PlayerController.GetInputAnalogKeyState` _controller "Gamepad_LeftY"))
  (bind _returnvalue_8 (`PlayerController.GetInputAnalogKeyState` _controller "Gamepad_RightX"))
  (`|ExecutionSequence`
    (:`then_0`
      (if (`PlayerController.IsInputKeyDown` _controller "Gamepad_FaceButton_Bottom")
        (`/Engine/EditorBlueprintResources/StandardMacros.DoOnce` false :!label _label
          (:`Completed`
            (`self.Input_A` (`self.PlayerNumber`))))
        (else
          (goto _label :!via `Reset`))))
    (:`then_1`
      (if (`PlayerController.IsInputKeyDown` _controller "Gamepad_FaceButton_Right")
        (`/Engine/EditorBlueprintResources/StandardMacros.DoOnce` false :!label _label_2
          (:`Completed`
            (`self.Input_B` (`self.PlayerNumber`))))
        (else
          (goto _label_2 :!via `Reset`))))
    (:`then_2`
      (if (`PlayerController.IsInputKeyDown` _controller "Gamepad_Special_Right")
        (`/Engine/EditorBlueprintResources/StandardMacros.DoOnce` false :!label _label_3
          (:`Completed`
            (`self.Input_Start` (`self.Controller`))))
        (else
          (goto _label_3 :!via `Reset`))))
    (:`then_3`
      (if (>= _returnvalue 0.9)
        (`/Engine/EditorBlueprintResources/StandardMacros.DoOnce` false :!label _label_4
          (:`Completed`
            (`self.Input_UP_L` (`self.PlayerNumber`))))
        (elif (< _returnvalue 0.6)
          (goto _label_4 :!via `Reset`))))
    (:`then_4`
      (if (<= _returnvalue_7 -0.9)
        (`/Engine/EditorBlueprintResources/StandardMacros.DoOnce` false :!label _label_5
          (:`Completed`
            (`self.Input_Down_L` (`self.PlayerNumber`))))
        (elif (> _returnvalue_7 -0.6)
          (goto _label_5 :!via `Reset`))))
    (:`then_5`
      (if (>= _returnvalue_2 0.9)
        (`/Engine/EditorBlueprintResources/StandardMacros.DoOnce` false :!label _label_6
          (:`Completed`
            (`self.Input_UP_R` (`self.PlayerNumber`))))
        (elif (< _returnvalue_2 0.6)
          (goto _label_6 :!via `Reset`))))
    (:`then_6`
      (if (<= _returnvalue_3 -0.9)
        (`/Engine/EditorBlueprintResources/StandardMacros.DoOnce` false :!label _label_7
          (:`Completed`
            (`self.Input_Down_R` (`self.PlayerNumber`))))
        (elif (> _returnvalue_3 -0.6)
          (goto _label_7 :!via `Reset`))))
    (:`then_7`
      (if (>= _returnvalue_5 0.9)
        (`/Engine/EditorBlueprintResources/StandardMacros.DoOnce` false :!label _label_8
          (:`Completed`
            (`self.Input_Left_L` (`self.PlayerNumber`))))
        (elif (< _returnvalue_5 0.6)
          (goto _label_8 :!via `Reset`))))
    (:`then_8`
      (if (<= _returnvalue_6 -0.9)
        (`/Engine/EditorBlueprintResources/StandardMacros.DoOnce` false :!label _label_9
          (:`Completed`
            (`self.Input_Right_L` (`self.PlayerNumber`))))
        (elif (> _returnvalue_6 -0.6)
          (goto _label_9 :!via `Reset`))))
    (:`then_9`
      (if (>= _returnvalue_4 0.9)
        (`/Engine/EditorBlueprintResources/StandardMacros.DoOnce` false :!label _label_10
          (:`Completed`
            (`self.Input_Left_R` (`self.PlayerNumber`))))
        (elif (< _returnvalue_4 0.6)
          (goto _label_10 :!via `Reset`))))
    (:`then_10`
      (if (<= _returnvalue_8 -0.9)
        (`/Engine/EditorBlueprintResources/StandardMacros.DoOnce` false :!label _label_11
          (:`Completed`
            (`self.Input_Right_R` (`self.PlayerNumber`))))
        (elif (> _returnvalue_8 -0.6)
          (goto _label_11 :!via `Reset`))))))

(fn `GetPlayer`
  (returns (Player :type "/Game/Character/BP_Owner Object Reference"))
  (bind _player (`self.Player`))
  (`/Engine/EditorBlueprintResources/StandardMacros.IsValid` _player
    (:`Is Valid`
      _)
    (:`Is Not Valid`
      (set `self.Player` (`|GetArrayItem` (`/Game/GameInstance/MyGameInstance.Players` (cast `/Game/GameInstance/MyGameInstance` (`GameplayStatics.GetGameInstance`) :!pure true)) (`self.PlayerNumber`)))))
  (return _player))

(fn `UserConstructionScript`)