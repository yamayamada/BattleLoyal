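; BP_WallCreate is an actor that builds an invisible circular barrier, apparently to enclose a play area on the map.
; On BeginPlay it loops Num times, spacing tall box components evenly around a fixed-radius ring using FAddition on a unit vector and the step angle.
; Each box is yawed to its angle, hidden in game and set to the BlockAll collision profile.
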(event `self.ReceiveBeginPlay`
  (bind _num (`self.num`))
  (for _index (range _num)
    (bind _returnvalue (* (/ 360.0 (`KismetMathLibrary.Conv_IntToDouble` _num)) (`KismetMathLibrary.Conv_IntToDouble` _index)))
    (bind (_returnvalue_x _returnvalue_y) (`KismetMathLibrary.BreakVector2D` (* (`/Game/Math/BPF_Math.f_Addition` (1.0 0.0) _returnvalue) 1050.0)))
    (bind _returnvalue_2 (`AddComponent|NODE_AddBoxComponent-0` :`RelativeTransform` (`KismetMathLibrary.MakeTransform` (`KismetMathLibrary.MakeVector` _returnvalue_x _returnvalue_y) (`KismetMathLibrary.MakeRotator` 0.0 0.0 _returnvalue) (1.0 1.0 10.0))))
    (`SceneComponent.SetHiddenInGame` _returnvalue_2 true false)
    (`PrimitiveComponent.SetCollisionProfileName` _returnvalue_2 "BlockAll")))

(fn `UserConstructionScript`)