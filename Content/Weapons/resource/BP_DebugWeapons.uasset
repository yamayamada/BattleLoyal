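; BP_DebugWeapons is a debug weapons actor that moves in a straight line once play begins.
; BeginPlay caches the forward vector of its Sphere component and the actor's starting location.
; Tick adds that direction times Speed to the stored position and sets the location without sweep or DeltaSeconds scaling, so travel is frame-rate dependent.
; It has no active overlap or hit logic.
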(event `self.ReceiveBeginPlay`
  (`parent.ReceiveBeginPlay`)
  (set `self.Move` (`SceneComponent.GetForwardVector` (`self.Sphere`)))
  (set `self.position` (`self.K2_GetActorLocation`)))

(event `self.ReceiveTick`
  (params (DeltaSeconds :type "Float (single-precision)"))
  (`parent.ReceiveTick` DeltaSeconds)
  (bind _output_get (set `self.position` (+ (`self.position`) (* (`self.Move`) (`self.speed`)))))
  (`self.K2_SetActorLocation` _output_get))

(fn `UserConstructionScript`
  (`parent.UserConstructionScript`))