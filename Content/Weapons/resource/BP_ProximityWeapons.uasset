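; Proximity (melee) weapon Blueprint that opens and closes an attack hit window by toggling AttackCollision.
; AttackON enables query and physics collision, and AttackOFF disables it.
; Two DoOnce nodes re-arm each other as a latch, so repeated calls to the same event are ignored.
; Hit handling is unfinished: the overlap event is empty, and the BP_Owner cast with its self-hit check is disconnected.
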(event `AttackON`
  (bind _attackcollision (`self.AttackCollision`))
  (`/Engine/EditorBlueprintResources/StandardMacros.DoOnce` false :!label _label
    (:`Completed`
      (`PrimitiveComponent.SetCollisionEnabled` _attackcollision "QueryAndPhysics")
      (goto _label_2 :!via `Reset`))))

(event `AttackOFF`
  (`/Engine/EditorBlueprintResources/StandardMacros.DoOnce` false :!label _label_2
    (:`Completed`
      (`PrimitiveComponent.SetCollisionEnabled` (`self.AttackCollision`) "NoCollision")
      (goto _label :!via `Reset`))))

(event `self.AttackCollision.OnComponentBeginOverlap`
  (params (OverlappedComponent :type "PrimitiveComponent Object Reference") (OtherActor :type "Actor Object Reference") (OtherComp :type "PrimitiveComponent Object Reference") (OtherBodyIndex :type Integer) (bFromSweep :type Boolean) (SweepResult :type "HitResult Structure (by ref)")))

(fn `UserConstructionScript`)