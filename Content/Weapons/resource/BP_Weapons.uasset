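; BP_Weapons is a weapon actor Blueprint that tracks an elapsed time against a limit.
; BeginPlay caches the root component's forward vector and zeroes the timer.
; UpdateTime adds to the timer, TimeOut reports whether it has reached LimitTime, TimeParsent returns the elapsed fraction, and Reset clears it.
; Tick and overlap events are disabled, and nothing in this Blueprint calls the timer functions or uses the cached direction.
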(event `self.ReceiveBeginPlay`
  (set `self.Forward` (`SceneComponent.GetForwardVector` (`self.DefaultSceneRoot`)))
  (set `self.Time` 0.0))

(fn `Reset`
  (set `self.Time` 0.0))

(fn `TimeOut`
  (returns (isTimeOut :type Boolean))
  (return (<= (`self.LimitTime`) (`self.Time`))))

(fn `TimeParsent`
  (returns (Parsent :type "Float (double-precision)"))
  (return (/ (`self.Time`) (`self.LimitTime`))))

(fn `UpdateTime`
  (params (Time :type "Float (double-precision)"))
  (set `self.Time` (+ Time (`self.Time`))))

(fn `UserConstructionScript`)