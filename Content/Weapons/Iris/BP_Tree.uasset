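; Tree actor for the Iris weapon that grows, topples and damages BP_Owner characters other than the player who fired it.
; Two chained timelines animate growth as a stretch-and-settle scale, and a third rolls the tree mesh over, then resets its rotation and shrinks the actor.
; Capsule overlaps deal fixed damage, with paired DoOnce gates in AttackON and AttackOFF toggling collision, which is switched off at BeginPlay.
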(event `WoodGlowStart`
  (bind _xyscale (`self.XYScale`))
  (bind (_direction _time) (`Timeline|WoodGlowTick` :!via `PlayFromStart` :!label _label)
    (:`Update`
      (set `self.ZScale` (`KismetMathLibrary.Lerp` 0.0 1.2 _time))
      (set `self.XYScale` (`KismetMathLibrary.Lerp` 1.0 0.5 _time))
      (if (<= _time 0.99)
        (`self.SetActorScale3D` (`KismetMathLibrary.MakeVector` _xyscale _xyscale (`self.ZScale`)))))
    (:`Finished`
      (`self.WoodGlowEnd`)
      (`self.WoodGlow2Start`))))

(event `WoodGlowEnd`
  (goto _label :!via `Stop`))

(event `WoodGlow2Start`
  (bind _xyscale (`self.XYScale`))
  (bind (_direction _time) (`Timeline|WoodGlow2Tick` :!via `PlayFromStart` :!label _label_2)
    (:`Update`
      (set `self.ZScale` (`KismetMathLibrary.Lerp` 1.2 1.0 _time))
      (set `self.XYScale` (`KismetMathLibrary.Lerp` 0.5 1.0 _time))
      (if (<= _time 0.99)
        (`self.SetActorScale3D` (`KismetMathLibrary.MakeVector` _xyscale _xyscale (`self.ZScale`)))))
    (:`Finished`
      (`self.WoodGlow2End`))))

(event `WoodGlow2End`
  (goto _label_2 :!via `Stop`))

(event `WoodFallDownStart`
  (bind (_direction _time) (`Timeline|WoodFallDownTick` :!via `PlayFromStart` :!label _label_3)
    (:`Update`
      (bind _output_get (set `self.RotateTree` _time))
      (if (<= _output_get 90.0)
        (`SceneComponent.K2_SetRelativeRotation` (`self.TX_iris_weapon_tree_B`) (`KismetMathLibrary.MakeRotator` (`self.RotateTree`)) false false)))
    (:`Finished`
      (`self.WoodFallDownEnd`)
      (`SceneComponent.K2_SetRelativeRotation` (`self.TX_iris_weapon_tree_B`) (`KismetMathLibrary.MakeRotator` 0.0) false false)
      (`self.SetActorScale3D` (0.1 0.1 0.1)))))

(event `WoodFallDownEnd`
  (goto _label_3 :!via `Stop`))

(event `self.Capsule.OnComponentBeginOverlap`
  (params (OverlappedComponent :type "PrimitiveComponent Object Reference") (OtherActor :type "Actor Object Reference") (OtherComp :type "PrimitiveComponent Object Reference") (OtherBodyIndex :type Integer) (bFromSweep :type Boolean) (SweepResult :type "HitResult Structure (by ref)"))
  (bind _asbp_owner (cast `/Game/Character/BP_Owner` OtherActor))
  (if (!= _asbp_owner (`self.FirePlayer`))
    (`/Game/Character/BP_Owner.SendDamage` _asbp_owner _asbp_owner 50.0)))

(event `AttackON`
  (bind _capsule (`self.Capsule`))
  (`/Engine/EditorBlueprintResources/StandardMacros.DoOnce` false :!label _label_4
    (:`Completed`
      (`PrimitiveComponent.SetCollisionProfileName` _capsule "OverlapAllDynamic")
      (goto _label_5 :!via `Reset`))))

(event `self.ReceiveBeginPlay`
  (`self.AttackOFF`))

(event `AttackOFF`
  (`/Engine/EditorBlueprintResources/StandardMacros.DoOnce` false :!label _label_5
    (:`Completed`
      (`PrimitiveComponent.SetCollisionProfileName` (`self.Capsule`) "NoCollision")
      (goto _label_4 :!via `Reset`))))

(fn `UserConstructionScript`)