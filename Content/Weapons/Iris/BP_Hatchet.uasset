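; BP_Hatchet is a thrown hatchet projectile in the Iris weapons folder.
; Each tick it slightly rotates the actor, spins its Cube component and moves along the Forward variable by Speed without sweep or delta-time scaling.
; Its Sphere overlap destroys it on touching any BP_Owner other than a valid FirePlayer, with no damage applied here.
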(event `self.ReceiveBeginPlay`
  (`parent.ReceiveBeginPlay`))

(event `self.ReceiveTick`
  (params (DeltaSeconds :type "Float (single-precision)"))
  (`parent.ReceiveTick` DeltaSeconds)
  (`self.K2_AddActorWorldRotation` (struct :`Roll` 1.0))
  (`SceneComponent.K2_AddLocalRotation` (`self.Cube`) (struct :`Yaw` 15.0) false false)
  (`self.K2_SetActorLocation` (+ (`self.K2_GetActorLocation`) (* (`self.Forward`) (`self.Speed`)))))

(event `self.Sphere.OnComponentBeginOverlap`
  (params (OverlappedComponent :type "PrimitiveComponent Object Reference") (OtherActor :type "Actor Object Reference") (OtherComp :type "PrimitiveComponent Object Reference") (OtherBodyIndex :type Integer) (bFromSweep :type Boolean) (SweepResult :type "HitResult Structure (by ref)"))
  (bind _fireplayer (`self.FirePlayer`))
  (if (`KismetSystemLibrary.IsValid` _fireplayer)
    (bind _asbp_owner (cast `/Game/Character/BP_Owner` OtherActor))
    (if (not (== _asbp_owner _fireplayer))
      (`self.K2_DestroyActor`))))

(fn `UserConstructionScript`
  (`parent.UserConstructionScript`))