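; BP_Frypan is a spinning frying pan weapon that flies out from FirePlayer and comes back like a boomerang.
; Tick drives three modes: Forward decelerates over LimitTime, Hold hovers while the gamepad top face button stays held, and Return accelerates to a capped speed.
; The return direction is taken once toward FirePlayer's position, so it does not home.
; Overlapping any BP_Owner destroys the pan, as both branches of the owner check do the same.
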(event `self.ReceiveBeginPlay`
  (`parent.ReceiveBeginPlay`)
  (set `self.ForwardMove` (`SceneComponent.GetForwardVector` (`self.DefaultSceneRoot`)))
  (set `self.Position` (`self.K2_GetActorLocation`))
  (set `self.Time` (`self.LimitTime`)))

(event `self.ReceiveTick`
  (params (DeltaSeconds :type "Float (single-precision)"))
  (bind _returnvalue (+ (`self.Speed`) 0.5))
  (`parent.ReceiveTick` DeltaSeconds)
  (set `self.Time` (- (`self.Time`) DeltaSeconds))
  (`self.K2_AddActorWorldRotation` (struct :`Yaw` 5.0))
  (switch `/Game/Weapons/Cook/E_FrypanMode` (`self.Mode`)
    (:`NewEnumerator0`
      (if (<= (`self.Time`) 0.0)
        (set `self.Mode` "NewEnumerator1")
        (else
          (bind _output_get (set `self.Position` (+ (`self.Position`) (* (`self.ForwardMove`) (* (`self.Speed`) (/ (`self.Time`) (`self.LimitTime`)))))))
          (`self.K2_SetActorLocation` _output_get)))
      (if (<= (`PlayerController.GetInputAnalogKeyState` (cast `PlayerController` (`Pawn.GetController` (`self.FirePlayer`)) :!pure true) "Gamepad_FaceButton_Top") 0.9) :!label _label
        (set `self.ButtonFlg` false)))
    (:`NewEnumerator1`
      (if (`self.ButtonFlg`)
        (goto _label)
        (else
          (set `self.Mode` "NewEnumerator2")
          (set `self.ReturnMove` (`KismetMathLibrary.Normal` (- (`self.K2_GetActorLocation` (`self.FirePlayer`)) (`self.K2_GetActorLocation`)))))))
    (:`NewEnumerator2`
      (if (<= _returnvalue 5.0)
        (set `self.Speed` _returnvalue))
      (bind _output_get_2 (set `self.Position` (+ (`self.Position`) (* (`self.ReturnMove`) (`self.Speed`)))))
      (`self.K2_SetActorLocation` _output_get_2))))

(event `self.Sphere.OnComponentBeginOverlap`
  (params (OverlappedComponent :type "PrimitiveComponent Object Reference") (OtherActor :type "Actor Object Reference") (OtherComp :type "PrimitiveComponent Object Reference") (OtherBodyIndex :type Integer) (bFromSweep :type Boolean) (SweepResult :type "HitResult Structure (by ref)"))
  (bind _asbp_owner (cast `/Game/Character/BP_Owner` OtherActor))
  (if (and (== _asbp_owner (`self.FirePlayer`)) (`|EnumInequality` (`self.Mode`) "NewEnumerator0"))
    (`self.K2_DestroyActor`)
    (else
      (`self.K2_DestroyActor`))))

(fn `UserConstructionScript`
  (`parent.UserConstructionScript`))