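; BP_Dish is a thrown cooking-weapon projectile made of three spinning dish meshes.
; Until its timer runs out, Tick spreads the dishes along Forward on a sine height arc, staggered by array index, then pushes them onward and downward.
; Each box overlap with a BP_Owner other than FirePlayer removes and destroys that dish.
; After timeout, the actor destroys itself once the Cube dish's height reaches a low world threshold.
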(event `self.ReceiveBeginPlay`
  (`parent.ReceiveBeginPlay`)
  (set `self.LimitTime` 0.7)
  (set `self.HeightLange` 100.0)
  (set `self.BulletLange` 300.0)
  (set `self.Dishes` (`|MakeArray` (`self.StaticMesh1`) (`self.StaticMesh`) (`self.Cube`)))
  (set `self.BasePosition` (`self.K2_GetActorLocation`)))

(event `self.ReceiveTick`
  (params (DeltaSeconds :type "Float (single-precision)"))
  (bind _parsent (`self.TimeParsent`))
  (bind (_baseposition_x _baseposition_y _baseposition_z) (`KismetMathLibrary.BreakVector` (`self.BasePosition`)))
  (bind (_forward_x _forward_y) (`KismetMathLibrary.BreakVector` (`self.Forward`)))
  (bind (_forward_x_2 _forward_y_2) (`KismetMathLibrary.BreakVector` (`self.Forward`)))
  (bind (_returnvalue_x _returnvalue_y _returnvalue_z) (`KismetMathLibrary.BreakVector` (`SceneComponent.K2_GetComponentLocation` (`self.Cube`))))
  (bind _returnvalue (* _parsent (`self.BulletLange`)))
  (`parent.ReceiveTick` DeltaSeconds)
  (`self.UpdateTime` DeltaSeconds)
  (if (`self.TimeOut`)
    (for _array_element (`self.Dishes`)
      (`SceneComponent.K2_AddLocalRotation` _array_element (struct :`Pitch` -4.0) false false)
      (`SceneComponent.K2_AddWorldOffset` _array_element (`KismetMathLibrary.MakeVector` (* _forward_x_2 1.5) (* _forward_y_2 1.5) -3.0) false false))
    (if (<= _returnvalue_z -20.0)
      (`self.K2_DestroyActor`))
    (else
      (for (_array_element_2 _array_index) (`self.Dishes`)
        (`SceneComponent.K2_AddLocalRotation` _array_element_2 (struct :`Pitch` -4.0) false false)
        (bind _returnvalue_2 (`KismetMathLibrary.Conv_IntToDouble` _array_index))
        (bind _returnvalue_3 (/ (+ _returnvalue_2 1.0) 3.0))
        (`SceneComponent.K2_SetWorldLocation` _array_element_2 (`KismetMathLibrary.MakeVector` (+ (* _returnvalue_3 (* _returnvalue _forward_x)) _baseposition_x) (+ (* _returnvalue_3 (* _returnvalue _forward_y)) _baseposition_y) (+ (* (`KismetMathLibrary.DegSin` (* _parsent 180.0)) (`self.HeightLange`)) (+ _baseposition_z (* _returnvalue_2 10.0)))) false false)))))

(event `self.Box2.OnComponentBeginOverlap`
  (params (OverlappedComponent :type "PrimitiveComponent Object Reference") (OtherActor :type "Actor Object Reference") (OtherComp :type "PrimitiveComponent Object Reference") (OtherBodyIndex :type Integer) (bFromSweep :type Boolean) (SweepResult :type "HitResult Structure (by ref)"))
  (bind _staticmesh1 (`self.StaticMesh1`))
  (bind _fireplayer (`self.FirePlayer`))
  (`/Engine/EditorBlueprintResources/StandardMacros.IsValid` _fireplayer
    (:`Is Valid`
      (bind _asbp_owner (cast `/Game/Character/BP_Owner` OtherActor))
      (if (!= _asbp_owner _fireplayer)
        (`KismetArrayLibrary.Array_RemoveItem` (`self.Dishes`) _staticmesh1)
        (`ActorComponent.K2_DestroyComponent` _staticmesh1)))))

(event `self.Box1.OnComponentBeginOverlap`
  (params (OverlappedComponent :type "PrimitiveComponent Object Reference") (OtherActor :type "Actor Object Reference") (OtherComp :type "PrimitiveComponent Object Reference") (OtherBodyIndex :type Integer) (bFromSweep :type Boolean) (SweepResult :type "HitResult Structure (by ref)"))
  (bind _fireplayer (`self.FirePlayer`))
  (bind _staticmesh (`self.StaticMesh`))
  (`/Engine/EditorBlueprintResources/StandardMacros.IsValid` _fireplayer
    (:`Is Valid`
      (bind _asbp_owner (cast `/Game/Character/BP_Owner` OtherActor))
      (if (!= _asbp_owner _fireplayer)
        (`KismetArrayLibrary.Array_RemoveItem` (`self.Dishes`) _staticmesh)
        (`ActorComponent.K2_DestroyComponent` _staticmesh)))))

(event `self.Box.OnComponentBeginOverlap`
  (params (OverlappedComponent :type "PrimitiveComponent Object Reference") (OtherActor :type "Actor Object Reference") (OtherComp :type "PrimitiveComponent Object Reference") (OtherBodyIndex :type Integer) (bFromSweep :type Boolean) (SweepResult :type "HitResult Structure (by ref)"))
  (bind _cube (`self.Cube`))
  (bind _fireplayer (`self.FirePlayer`))
  (`/Engine/EditorBlueprintResources/StandardMacros.IsValid` _fireplayer
    (:`Is Valid`
      (bind _asbp_owner (cast `/Game/Character/BP_Owner` OtherActor))
      (if (!= _asbp_owner _fireplayer)
        (`KismetArrayLibrary.Array_RemoveItem` (`self.Dishes`) _cube)
        (`ActorComponent.K2_DestroyComponent` _cube)))))

(fn `UserConstructionScript`
  (`parent.UserConstructionScript`))