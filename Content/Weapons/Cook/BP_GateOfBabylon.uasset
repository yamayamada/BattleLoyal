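; Gate of Babylon weapon actor that drops a volley of dish meshes to damage players other than the one who fired it.
; BeginPlay gathers the root's static mesh children into the Dish array.
; Tick runs a timed Mode sequence: wait, lower each dish along local Z until it reaches world zero, pause, then destroy the actor.
; Duplicated per-box overlap events destroy their paired mesh and damage any BP_Owner except FirePlayer.
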(event `self.ReceiveBeginPlay`
  (`parent.ReceiveBeginPlay`)
  (for _array_element (`SceneComponent.GetChildrenComponents` (`self.DefaultSceneRoot`) false)
    (bind _asstatic_mesh_component (cast `StaticMeshComponent` _array_element))
    (`KismetArrayLibrary.Array_Add` (`self.Dish`) _asstatic_mesh_component)
    (set `self.LimitTime` 0.5)))

(event `self.ReceiveTick`
  (params (DeltaSeconds :type "Float (single-precision)"))
  (`parent.ReceiveTick` DeltaSeconds)
  (`self.UpdateTime` DeltaSeconds)
  (switch `int` (`self.Mode`)
    (:`0`
      (if (`self.TimeOut`)
        (`/Engine/EditorBlueprintResources/StandardMacros.IncrementInt` (`self.Mode`)
          (:`  `
            (`self.Reset`)
            (set `self.LimitTime` 1.5)))))
    (:`1`
      (for _array_element (`self.Dish`)
        (bind (_returnvalue_x _returnvalue_y _returnvalue_z) (`KismetMathLibrary.BreakVector` (`SceneComponent.K2_GetComponentLocation` _array_element)))
        (if (not (<= _returnvalue_z 0.0))
          (`SceneComponent.K2_AddLocalOffset` _array_element (* (0.0 0.0 -1.0) 20.0) false false)))
      (if (`self.TimeOut`)
        (`/Engine/EditorBlueprintResources/StandardMacros.IncrementInt` (`self.Mode`)
          (:`  `
            (`self.Reset`)
            (set `self.LimitTime` 0.5)))))
    (:`2`
      (if (`self.TimeOut`)
        (`/Engine/EditorBlueprintResources/StandardMacros.IncrementInt` (`self.Mode`)
          (:`  `
            (`self.K2_DestroyActor`)))))))

(event `self.Box17.OnComponentBeginOverlap`
  (params (OverlappedComponent :type "PrimitiveComponent Object Reference") (OtherActor :type "Actor Object Reference") (OtherComp :type "PrimitiveComponent Object Reference") (OtherBodyIndex :type Integer) (bFromSweep :type Boolean) (SweepResult :type "HitResult Structure (by ref)"))
  (bind _staticmesh16 (`self.StaticMesh16`))
  (bind _fireplayer (`self.FirePlayer`))
  (`/Engine/EditorBlueprintResources/StandardMacros.IsValid` _fireplayer
    (:`Is Valid`
      (bind _asbp_owner (cast `/Game/Character/BP_Owner` OtherActor))
      (if (not (== _asbp_owner _fireplayer))
        (`ActorComponent.K2_DestroyComponent` _staticmesh16)
        (`KismetArrayLibrary.Array_RemoveItem` (`self.Dish`) _staticmesh16)
        (`/Game/Character/BP_Owner.SendDamage` _asbp_owner _asbp_owner 20.0)))))

(event `self.Box16.OnComponentBeginOverlap`
  (params (OverlappedComponent :type "PrimitiveComponent Object Reference") (OtherActor :type "Actor Object Reference") (OtherComp :type "PrimitiveComponent Object Reference") (OtherBodyIndex :type Integer) (bFromSweep :type Boolean) (SweepResult :type "HitResult Structure (by ref)"))
  (bind _fireplayer (`self.FirePlayer`))
  (bind _staticmesh15 (`self.StaticMesh15`))
  (`/Engine/EditorBlueprintResources/StandardMacros.IsValid` _fireplayer
    (:`Is Valid`
      (bind _asbp_owner (cast `/Game/Character/BP_Owner` OtherActor))
      (if (not (== _asbp_owner _fireplayer))
        (`ActorComponent.K2_DestroyComponent` _staticmesh15)
        (`KismetArrayLibrary.Array_RemoveItem` (`self.Dish`) _staticmesh15)
        (`/Game/Character/BP_Owner.SendDamage` _asbp_owner _asbp_owner 20.0)))))

(event `self.Box15.OnComponentBeginOverlap`
  (params (OverlappedComponent :type "PrimitiveComponent Object Reference") (OtherActor :type "Actor Object Reference") (OtherComp :type "PrimitiveComponent Object Reference") (OtherBodyIndex :type Integer) (bFromSweep :type Boolean) (SweepResult :type "HitResult Structure (by ref)"))
  (bind _fireplayer (`self.FirePlayer`))
  (bind _staticmesh14 (`self.StaticMesh14`))
  (`/Engine/EditorBlueprintResources/StandardMacros.IsValid` _fireplayer
    (:`Is Valid`
      (bind _asbp_owner (cast `/Game/Character/BP_Owner` OtherActor))
      (if (not (== _asbp_owner _fireplayer))
        (`ActorComponent.K2_DestroyComponent` _staticmesh14)
        (`KismetArrayLibrary.Array_RemoveItem` (`self.Dish`) _staticmesh14)
        (`/Game/Character/BP_Owner.SendDamage` _asbp_owner _asbp_owner 20.0)))))

(event `self.Box14.OnComponentBeginOverlap`
  (params (OverlappedComponent :type "PrimitiveComponent Object Reference") (OtherActor :type "Actor Object Reference") (OtherComp :type "PrimitiveComponent Object Reference") (OtherBodyIndex :type Integer) (bFromSweep :type Boolean) (SweepResult :type "HitResult Structure (by ref)"))
  (bind _fireplayer (`self.FirePlayer`))
  (bind _staticmesh13 (`self.StaticMesh13`))
  (`/Engine/EditorBlueprintResources/StandardMacros.IsValid` _fireplayer
    (:`Is Valid`
      (bind _asbp_owner (cast `/Game/Character/BP_Owner` OtherActor))
      (if (not (== _asbp_owner _fireplayer))
        (`ActorComponent.K2_DestroyComponent` _staticmesh13)
        (`KismetArrayLibrary.Array_RemoveItem` (`self.Dish`) _staticmesh13)
        (`/Game/Character/BP_Owner.SendDamage` _asbp_owner _asbp_owner 20.0)))))

(event `self.Box13.OnComponentBeginOverlap`
  (params (OverlappedComponent :type "PrimitiveComponent Object Reference") (OtherActor :type "Actor Object Reference") (OtherComp :type "PrimitiveComponent Object Reference") (OtherBodyIndex :type Integer) (bFromSweep :type Boolean) (SweepResult :type "HitResult Structure (by ref)"))
  (bind _fireplayer (`self.FirePlayer`))
  (bind _staticmesh12 (`self.StaticMesh12`))
  (`/Engine/EditorBlueprintResources/StandardMacros.IsValid` _fireplayer
    (:`Is Valid`
      (bind _asbp_owner (cast `/Game/Character/BP_Owner` OtherActor))
      (if (not (== _asbp_owner _fireplayer))
        (`ActorComponent.K2_DestroyComponent` _staticmesh12)
        (`KismetArrayLibrary.Array_RemoveItem` (`self.Dish`) _staticmesh12)
        (`/Game/Character/BP_Owner.SendDamage` _asbp_owner _asbp_owner 20.0)))))

(event `self.Box12.OnComponentBeginOverlap`
  (params (OverlappedComponent :type "PrimitiveComponent Object Reference") (OtherActor :type "Actor Object Reference") (OtherComp :type "PrimitiveComponent Object Reference") (OtherBodyIndex :type Integer) (bFromSweep :type Boolean) (SweepResult :type "HitResult Structure (by ref)"))
  (bind _fireplayer (`self.FirePlayer`))
  (bind _staticmesh11 (`self.StaticMesh11`))
  (`/Engine/EditorBlueprintResources/StandardMacros.IsValid` _fireplayer
    (:`Is Valid`
      (bind _asbp_owner (cast `/Game/Character/BP_Owner` OtherActor))
      (if (not (== _asbp_owner _fireplayer))
        (`ActorComponent.K2_DestroyComponent` _staticmesh11)
        (`KismetArrayLibrary.Array_RemoveItem` (`self.Dish`) _staticmesh11)
        (`/Game/Character/BP_Owner.SendDamage` _asbp_owner _asbp_owner 20.0)))))

(event `self.Box11.OnComponentBeginOverlap`
  (params (OverlappedComponent :type "PrimitiveComponent Object Reference") (OtherActor :type "Actor Object Reference") (OtherComp :type "PrimitiveComponent Object Reference") (OtherBodyIndex :type Integer) (bFromSweep :type Boolean) (SweepResult :type "HitResult Structure (by ref)"))
  (bind _fireplayer (`self.FirePlayer`))
  (bind _staticmesh10 (`self.StaticMesh10`))
  (`/Engine/EditorBlueprintResources/StandardMacros.IsValid` _fireplayer
    (:`Is Valid`
      (bind _asbp_owner (cast `/Game/Character/BP_Owner` OtherActor))
      (if (not (== _asbp_owner _fireplayer))
        (`ActorComponent.K2_DestroyComponent` _staticmesh10)
        (`KismetArrayLibrary.Array_RemoveItem` (`self.Dish`) _staticmesh10)
        (`/Game/Character/BP_Owner.SendDamage` _asbp_owner _asbp_owner 20.0)))))

(event `self.Box10.OnComponentBeginOverlap`
  (params (OverlappedComponent :type "PrimitiveComponent Object Reference") (OtherActor :type "Actor Object Reference") (OtherComp :type "PrimitiveComponent Object Reference") (OtherBodyIndex :type Integer) (bFromSweep :type Boolean) (SweepResult :type "HitResult Structure (by ref)"))
  (bind _fireplayer (`self.FirePlayer`))
  (bind _staticmesh9 (`self.StaticMesh9`))
  (`/Engine/EditorBlueprintResources/StandardMacros.IsValid` _fireplayer
    (:`Is Valid`
      (bind _asbp_owner (cast `/Game/Character/BP_Owner` OtherActor))
      (if (not (== _asbp_owner _fireplayer))
        (`ActorComponent.K2_DestroyComponent` _staticmesh9)
        (`KismetArrayLibrary.Array_RemoveItem` (`self.Dish`) _staticmesh9)
        (`/Game/Character/BP_Owner.SendDamage` _asbp_owner _asbp_owner 20.0)))))

(event `self.Box9.OnComponentBeginOverlap`
  (params (OverlappedComponent :type "PrimitiveComponent Object Reference") (OtherActor :type "Actor Object Reference") (OtherComp :type "PrimitiveComponent Object Reference") (OtherBodyIndex :type Integer) (bFromSweep :type Boolean) (SweepResult :type "HitResult Structure (by ref)"))
  (bind _fireplayer (`self.FirePlayer`))
  (bind _staticmesh8 (`self.StaticMesh8`))
  (`/Engine/EditorBlueprintResources/StandardMacros.IsValid` _fireplayer
    (:`Is Valid`
      (bind _asbp_owner (cast `/Game/Character/BP_Owner` OtherActor))
      (if (not (== _asbp_owner _fireplayer))
        (`ActorComponent.K2_DestroyComponent` _staticmesh8)
        (`KismetArrayLibrary.Array_RemoveItem` (`self.Dish`) _staticmesh8)
        (`/Game/Character/BP_Owner.SendDamage` _asbp_owner _asbp_owner 20.0)))))

(event `self.Box8.OnComponentBeginOverlap`
  (params (OverlappedComponent :type "PrimitiveComponent Object Reference") (OtherActor :type "Actor Object Reference") (OtherComp :type "PrimitiveComponent Object Reference") (OtherBodyIndex :type Integer) (bFromSweep :type Boolean) (SweepResult :type "HitResult Structure (by ref)"))
  (bind _fireplayer (`self.FirePlayer`))
  (bind _staticmesh7 (`self.StaticMesh7`))
  (`/Engine/EditorBlueprintResources/StandardMacros.IsValid` _fireplayer
    (:`Is Valid`
      (bind _asbp_owner (cast `/Game/Character/BP_Owner` OtherActor))
      (if (not (== _asbp_owner _fireplayer))
        (`ActorComponent.K2_DestroyComponent` _staticmesh7)
        (`KismetArrayLibrary.Array_RemoveItem` (`self.Dish`) _staticmesh7)
        (`/Game/Character/BP_Owner.SendDamage` _asbp_owner _asbp_owner 20.0)))))

(event `self.Box7.OnComponentBeginOverlap`
  (params (OverlappedComponent :type "PrimitiveComponent Object Reference") (OtherActor :type "Actor Object Reference") (OtherComp :type "PrimitiveComponent Object Reference") (OtherBodyIndex :type Integer) (bFromSweep :type Boolean) (SweepResult :type "HitResult Structure (by ref)"))
  (bind _fireplayer (`self.FirePlayer`))
  (bind _staticmesh6 (`self.StaticMesh6`))
  (`/Engine/EditorBlueprintResources/StandardMacros.IsValid` _fireplayer
    (:`Is Valid`
      (bind _asbp_owner (cast `/Game/Character/BP_Owner` OtherActor))
      (if (not (== _asbp_owner _fireplayer))
        (`ActorComponent.K2_DestroyComponent` _staticmesh6)
        (`KismetArrayLibrary.Array_RemoveItem` (`self.Dish`) _staticmesh6)
        (`/Game/Character/BP_Owner.SendDamage` _asbp_owner _asbp_owner 20.0)))))

(event `self.Box6.OnComponentBeginOverlap`
  (params (OverlappedComponent :type "PrimitiveComponent Object Reference") (OtherActor :type "Actor Object Reference") (OtherComp :type "PrimitiveComponent Object Reference") (OtherBodyIndex :type Integer) (bFromSweep :type Boolean) (SweepResult :type "HitResult Structure (by ref)"))
  (bind _fireplayer (`self.FirePlayer`))
  (bind _staticmesh5 (`self.StaticMesh5`))
  (`/Engine/EditorBlueprintResources/StandardMacros.IsValid` _fireplayer
    (:`Is Valid`
      (bind _asbp_owner (cast `/Game/Character/BP_Owner` OtherActor))
      (if (not (== _asbp_owner _fireplayer))
        (`ActorComponent.K2_DestroyComponent` _staticmesh5)
        (`KismetArrayLibrary.Array_RemoveItem` (`self.Dish`) _staticmesh5)
        (`/Game/Character/BP_Owner.SendDamage` _asbp_owner _asbp_owner 20.0)))))

(event `self.Box5.OnComponentBeginOverlap`
  (params (OverlappedComponent :type "PrimitiveComponent Object Reference") (OtherActor :type "Actor Object Reference") (OtherComp :type "PrimitiveComponent Object Reference") (OtherBodyIndex :type Integer) (bFromSweep :type Boolean) (SweepResult :type "HitResult Structure (by ref)"))
  (bind _fireplayer (`self.FirePlayer`))
  (bind _staticmesh4 (`self.StaticMesh4`))
  (`/Engine/EditorBlueprintResources/StandardMacros.IsValid` _fireplayer
    (:`Is Valid`
      (bind _asbp_owner (cast `/Game/Character/BP_Owner` OtherActor))
      (if (not (== _asbp_owner _fireplayer))
        (`ActorComponent.K2_DestroyComponent` _staticmesh4)
        (`KismetArrayLibrary.Array_RemoveItem` (`self.Dish`) _staticmesh4)
        (`/Game/Character/BP_Owner.SendDamage` _asbp_owner _asbp_owner 20.0)))))

(event `self.Box4.OnComponentBeginOverlap`
  (params (OverlappedComponent :type "PrimitiveComponent Object Reference") (OtherActor :type "Actor Object Reference") (OtherComp :type "PrimitiveComponent Object Reference") (OtherBodyIndex :type Integer) (bFromSweep :type Boolean) (SweepResult :type "HitResult Structure (by ref)"))
  (bind _fireplayer (`self.FirePlayer`))
  (bind _staticmesh3 (`self.StaticMesh3`))
  (`/Engine/EditorBlueprintResources/StandardMacros.IsValid` _fireplayer
    (:`Is Valid`
      (bind _asbp_owner (cast `/Game/Character/BP_Owner` OtherActor))
      (if (not (== _asbp_owner _fireplayer))
        (`ActorComponent.K2_DestroyComponent` _staticmesh3)
        (`KismetArrayLibrary.Array_RemoveItem` (`self.Dish`) _staticmesh3)
        (`/Game/Character/BP_Owner.SendDamage` _asbp_owner _asbp_owner 20.0)))))

(event `self.Box3.OnComponentBeginOverlap`
  (params (OverlappedComponent :type "PrimitiveComponent Object Reference") (OtherActor :type "Actor Object Reference") (OtherComp :type "PrimitiveComponent Object Reference") (OtherBodyIndex :type Integer) (bFromSweep :type Boolean) (SweepResult :type "HitResult Structure (by ref)"))
  (bind _fireplayer (`self.FirePlayer`))
  (bind _staticmesh2 (`self.StaticMesh2`))
  (`/Engine/EditorBlueprintResources/StandardMacros.IsValid` _fireplayer
    (:`Is Valid`
      (bind _asbp_owner (cast `/Game/Character/BP_Owner` OtherActor))
      (if (not (== _asbp_owner _fireplayer))
        (`ActorComponent.K2_DestroyComponent` _staticmesh2)
        (`KismetArrayLibrary.Array_RemoveItem` (`self.Dish`) _staticmesh2)
        (`/Game/Character/BP_Owner.SendDamage` _asbp_owner _asbp_owner 20.0)))))

(event `self.Box2.OnComponentBeginOverlap`
  (params (OverlappedComponent :type "PrimitiveComponent Object Reference") (OtherActor :type "Actor Object Reference") (OtherComp :type "PrimitiveComponent Object Reference") (OtherBodyIndex :type Integer) (bFromSweep :type Boolean) (SweepResult :type "HitResult Structure (by ref)"))
  (bind _fireplayer (`self.FirePlayer`))
  (bind _staticmesh1 (`self.StaticMesh1`))
  (`/Engine/EditorBlueprintResources/StandardMacros.IsValid` _fireplayer
    (:`Is Valid`
      (bind _asbp_owner (cast `/Game/Character/BP_Owner` OtherActor))
      (if (not (== _asbp_owner _fireplayer))
        (`ActorComponent.K2_DestroyComponent` _staticmesh1)
        (`KismetArrayLibrary.Array_RemoveItem` (`self.Dish`) _staticmesh1)
        (`/Game/Character/BP_Owner.SendDamage` _asbp_owner _asbp_owner 20.0)))))

(event `self.Box1.OnComponentBeginOverlap`
  (params (OverlappedComponent :type "PrimitiveComponent Object Reference") (OtherActor :type "Actor Object Reference") (OtherComp :type "PrimitiveComponent Object Reference") (OtherBodyIndex :type Integer) (bFromSweep :type Boolean) (SweepResult :type "HitResult Structure (by ref)"))
  (bind _fireplayer (`self.FirePlayer`))
  (bind _staticmesh (`self.StaticMesh`))
  (`/Engine/EditorBlueprintResources/StandardMacros.IsValid` _fireplayer
    (:`Is Valid`
      (bind _asbp_owner (cast `/Game/Character/BP_Owner` OtherActor))
      (if (not (== _asbp_owner _fireplayer))
        (`ActorComponent.K2_DestroyComponent` _staticmesh)
        (`KismetArrayLibrary.Array_RemoveItem` (`self.Dish`) _staticmesh)
        (`/Game/Character/BP_Owner.SendDamage` _asbp_owner _asbp_owner 20.0)))))

(event `self.Box.OnComponentBeginOverlap`
  (params (OverlappedComponent :type "PrimitiveComponent Object Reference") (OtherActor :type "Actor Object Reference") (OtherComp :type "PrimitiveComponent Object Reference") (OtherBodyIndex :type Integer) (bFromSweep :type Boolean) (SweepResult :type "HitResult Structure (by ref)"))
  (bind _cube (`self.Cube`))
  (bind _fireplayer (`self.FirePlayer`))
  (`/Engine/EditorBlueprintResources/StandardMacros.IsValid` _fireplayer
    (:`Is Valid`
      (bind _asbp_owner (cast `/Game/Character/BP_Owner` OtherActor))
      (if (not (== _asbp_owner _fireplayer))
        (`ActorComponent.K2_DestroyComponent` _cube)
        (`KismetArrayLibrary.Array_RemoveItem` (`self.Dish`) _cube)
        (`/Game/Character/BP_Owner.SendDamage` _asbp_owner _asbp_owner 20.0)))))

(fn `UserConstructionScript`
  (`parent.UserConstructionScript`))