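; BP_Missil is a missile that picks a target among BP_Owner players other than the one who fired it.
; Until TimeOut is true, Tick picks the nearest player (the dot-product filter always passes) and sets yaw from dot and cross products.
; After timeout it moves straight along its forward vector at Speed.
; Its box destroys it on overlapping another BP_Owner, with no damage applied here.
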(event `self.ReceiveBeginPlay`
  (bind _fireplayer (`self.FirePlayer`))
  (`parent.ReceiveBeginPlay`)
  (if (`KismetSystemLibrary.IsValid` _fireplayer) :!label _label
    (bind _outactors (`GameplayStatics.GetAllActorsOfClass` "/Game/Character/BP_Owner.BP_Owner_C"))
    (bind _output_get (set `self.Players` _outactors))
    (`KismetArrayLibrary.Array_RemoveItem` _output_get _fireplayer)
    (set `self.LimitTime` 0.5)
    (else
      (`KismetSystemLibrary.Delay` 0.01)
      (goto _label))))

(event `self.ReceiveTick`
  (params (DeltaSeconds :type "Float (single-precision)"))
  (bind _returnvalue (`KismetMathLibrary.Normal` (- (`self.K2_GetActorLocation` (`self.TargetActor`)) (`self.K2_GetActorLocation`))))
  (`parent.ReceiveTick` DeltaSeconds)
  (if (`self.TimeOut`)
    (`self.K2_SetActorLocation` (+ (`self.K2_GetActorLocation`) (* (`SceneComponent.GetForwardVector` (`self.DefaultSceneRoot`)) (`self.Speed`))))
    (else
      (`self.UpdateTime` DeltaSeconds)
      (set `self.TargetActor` null)
      (for _array_element (`self.Players`)
        (if (<= (`/Game/Math/BPF_Math.f_Dot3` (`SceneComponent.GetForwardVector` (`self.DefaultSceneRoot`)) (`KismetMathLibrary.Normal` (- (`self.K2_GetActorLocation` _array_element) (`self.K2_GetActorLocation`)))) 15.0)
          (`/Engine/EditorBlueprintResources/StandardMacros.IsValid` (`self.TargetActor`)
            (:`Is Valid`
              (if (not (<= (`KismetMathLibrary.VSize` (- (`self.K2_GetActorLocation` (`self.TargetActor`)) (`self.K2_GetActorLocation`))) (`KismetMathLibrary.VSize` (- (`self.K2_GetActorLocation` _array_element) (`self.K2_GetActorLocation`)))))
                (set `self.TargetActor` _array_element)))
            (:`Is Not Valid`
              (set `self.TargetActor` _array_element)))))
      (`/Engine/EditorBlueprintResources/StandardMacros.IsValid` (`self.TargetActor`)
        (:`Is Valid`
          (`self.K2_SetActorRotation` (`KismetMathLibrary.MakeRotator` 0.0 0.0 (* (`/Game/Math/BPF_Math.f_Dot3` (1.0 0.0 0.0) _returnvalue) (* (`/Game/Math/BPF_Math.f_Cross3` (1.0 0.0 0.0) _returnvalue) -1.0)))))))))

(event `self.Box.OnComponentBeginOverlap`
  (params (OverlappedComponent :type "PrimitiveComponent Object Reference") (OtherActor :type "Actor Object Reference") (OtherComp :type "PrimitiveComponent Object Reference") (OtherBodyIndex :type Integer) (bFromSweep :type Boolean) (SweepResult :type "HitResult Structure (by ref)"))
  (bind _fireplayer (`self.FirePlayer`))
  (`/Engine/EditorBlueprintResources/StandardMacros.IsValid` _fireplayer
    (:`Is Valid`
      (bind _asbp_owner (cast `/Game/Character/BP_Owner` OtherActor))
      (if (not (== _asbp_owner _fireplayer))
        (`self.K2_DestroyActor`)))))

(fn `UserConstructionScript`
  (`parent.UserConstructionScript`))