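; Weapon laser actor that extends a beam forward and deals fixed damage to any BP_Owner overlapping its box.
; Each tick it lengthens and advances the cylinder, rotates the root and, while live, spawns BP_LaserChild actors at four offset arrows.
; Once hit or expired, it shrinks to zero size, then destroys itself.
; Growth, movement and shrinking scale with frame time, while rotation and spawning run per tick.
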(event `self.ReceiveBeginPlay`
  (bind _size (`self.Size`))
  (`parent.ReceiveBeginPlay`)
  (`SceneComponent.SetWorldScale3D` (`self.Cylinder`) (`KismetMathLibrary.MakeVector` _size _size))
  (`SceneComponent.SetWorldScale3D` (`self.Sphere`) (`KismetMathLibrary.MakeVector` _size _size _size))
  (`SceneComponent.K2_AddLocalOffset` (`self.Arrow`) (`KismetMathLibrary.MakeVector` 0.0 (* (`self.Size`) 55.0)) false false)
  (`SceneComponent.K2_AddLocalOffset` (`self.Arrow1`) (`KismetMathLibrary.MakeVector` 0.0 (* (`self.Size`) -55.0)) false false)
  (`SceneComponent.K2_AddLocalOffset` (`self.Arrow2`) (`KismetMathLibrary.MakeVector` 0.0 0.0 (* (`self.Size`) 55.0)) false false)
  (`SceneComponent.K2_AddLocalOffset` (`self.Arrow3`) (`KismetMathLibrary.MakeVector` 0.0 0.0 (* (`self.Size`) -55.0)) false false))

(event `self.ReceiveTick`
  (params (DeltaSeconds :type "Float (single-precision)"))
  (bind _size (`self.Size`))
  (bind _size_2 (`self.Size`))
  (`parent.ReceiveTick` DeltaSeconds)
  (set `self.FrameFit` (/ DeltaSeconds 0.01))
  (set `self.LifeTime` (- (`self.LifeTime`) DeltaSeconds))
  (if (or (`self.IsHit`) (<= (`self.LifeTime`) 0.0))
    (if (<= (`self.Size`) 0.0)
      (`self.K2_DestroyActor`)
      (else
        (set `self.Size` (+ (`self.Size`) (* (`self.FrameFit`) -0.1)))
        (`SceneComponent.SetWorldScale3D` (`self.Sphere`) (`KismetMathLibrary.MakeVector` _size _size _size))
        (bind _output_get (set `self.LaserLength` (+ (`self.LaserLength`) (* (* (`self.Speed`) (`self.FrameFit`)) 0.1)) :!label _label))
        (`SceneComponent.SetWorldScale3D` (`self.Cylinder`) (`KismetMathLibrary.MakeVector` _size_2 _size_2 _output_get))
        (`SceneComponent.K2_SetWorldLocation` (`self.Cylinder`) (+ (`SceneComponent.K2_GetComponentLocation` (`self.Cylinder`)) (* (`SceneComponent.GetForwardVector` (`self.DefaultSceneRoot`)) (* (* (`self.Speed`) (`self.FrameFit`)) 5.0))) false false)
        (`SceneComponent.K2_AddLocalRotation` (`self.DefaultSceneRoot`) (struct :`Roll` -10.0) false false)))
    (else
      (`|SpawnActorFromClass` "/Game/Weapons/MID-3/BP_LaserChild.BP_LaserChild_C" (`SceneComponent.K2_GetComponentToWorld` (`self.Arrow`)) "Undefined" "OverrideRootScale" null null)
      (`|SpawnActorFromClass` "/Game/Weapons/MID-3/BP_LaserChild.BP_LaserChild_C" (`SceneComponent.K2_GetComponentToWorld` (`self.Arrow1`)) "Undefined" "OverrideRootScale" null null)
      (`|SpawnActorFromClass` "/Game/Weapons/MID-3/BP_LaserChild.BP_LaserChild_C" (`SceneComponent.K2_GetComponentToWorld` (`self.Arrow2`)) "Undefined" "OverrideRootScale" null null)
      (`|SpawnActorFromClass` "/Game/Weapons/MID-3/BP_LaserChild.BP_LaserChild_C" (`SceneComponent.K2_GetComponentToWorld` (`self.Arrow3`)) "Undefined" "OverrideRootScale" null null)
      (goto _label))))

(event `self.Box.OnComponentBeginOverlap`
  (params (OverlappedComponent :type "PrimitiveComponent Object Reference") (OtherActor :type "Actor Object Reference") (OtherComp :type "PrimitiveComponent Object Reference") (OtherBodyIndex :type Integer) (bFromSweep :type Boolean) (SweepResult :type "HitResult Structure (by ref)"))
  (bind _asbp_owner (cast `/Game/Character/BP_Owner` OtherActor))
  (`/Game/Character/BP_Owner.SendDamage` _asbp_owner _asbp_owner 50.0))

(fn `UserConstructionScript`
  (`parent.UserConstructionScript`))