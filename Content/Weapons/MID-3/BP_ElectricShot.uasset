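; Electric shot projectile for the MID-3 weapon, flying straight along its initial forward vector with a spinning aura.
; BeginPlay caches that direction and gives each child component of Sphere a random spin.
; Tick applies the spins and moves the actor by Speed per frame, without sweep or delta-time scaling.
; Sphere1 overlap destroys the shot on hitting a BP_Owner other than a valid FirePlayer; no damage is applied here.
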(event `self.ReceiveBeginPlay`
  (`parent.ReceiveBeginPlay`)
  (set `self.Move` (`SceneComponent.GetForwardVector` (`self.DefaultSceneRoot`)))
  (bind _output_get (set `self.Aura` (`SceneComponent.GetChildrenComponents` (`self.Sphere`) false)))
  (for _ _output_get
    (`KismetArrayLibrary.Array_Add` (`self.AuraRotation`) (`KismetMathLibrary.MakeRotator` (`KismetMathLibrary.RandomFloatInRange` -5.0 5.0) (`KismetMathLibrary.RandomFloatInRange` -5.0 5.0) (`KismetMathLibrary.RandomFloatInRange` -5.0 5.0)))))

(event `self.ReceiveActorBeginOverlap`
  (params (OtherActor :type "Actor Object Reference"))
  (`parent.ReceiveActorBeginOverlap` OtherActor))

(event `self.ReceiveTick`
  (params (DeltaSeconds :type "Float (single-precision)"))
  (`parent.ReceiveTick` DeltaSeconds)
  (for (_array_element _array_index) (`self.Aura`)
    (`SceneComponent.K2_AddLocalRotation` _array_element (`|GetArrayItem` (`self.AuraRotation`) _array_index) false false))
  (`self.K2_AddActorWorldOffset` (* (`self.Move`) (`self.Speed`))))

(event `self.Sphere1.OnComponentBeginOverlap`
  (params (OverlappedComponent :type "PrimitiveComponent Object Reference") (OtherActor :type "Actor Object Reference") (OtherComp :type "PrimitiveComponent Object Reference") (OtherBodyIndex :type Integer) (bFromSweep :type Boolean) (SweepResult :type "HitResult Structure (by ref)"))
  (bind _fireplayer (`self.FirePlayer`))
  (`/Engine/EditorBlueprintResources/StandardMacros.IsValid` _fireplayer
    (:`Is Valid`
      (bind _asbp_owner (cast `/Game/Character/BP_Owner` OtherActor))
      (if (not (== _asbp_owner _fireplayer))
        (`self.K2_DestroyActor`)))))

(fn `UserConstructionScript`
  (`parent.UserConstructionScript`))