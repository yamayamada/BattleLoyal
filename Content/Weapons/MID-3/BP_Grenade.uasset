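; Grenade projectile Actor that is lobbed along its Forward vector from its spawn position.
; Tick drives a timed sine arc while spinning the Sphere, using timer and percent helpers not defined here.
; After timeout it keeps moving forward and drops by fixed per-frame steps, destroying itself at or below world Z zero.
; Sphere1 overlap checks for a BP_Owner other than FirePlayer but takes no action.
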(event `self.ReceiveBeginPlay`
  (`parent.ReceiveBeginPlay`)
  (set `self.BasePosition` (`self.K2_GetActorLocation`))
  (`self.Reset`)
  (set `self.LimitTime` 0.5))

(event `self.ReceiveTick`
  (params (DeltaSeconds :type "Float (single-precision)"))
  (bind (_returnvalue_x _returnvalue_y _returnvalue_z) (`KismetMathLibrary.BreakVector` (`self.K2_GetActorLocation`)))
  (bind (_baseposition_x _baseposition_y _baseposition_z) (`KismetMathLibrary.BreakVector` (`self.BasePosition`)))
  (bind (_forward_x _forward_y) (`KismetMathLibrary.BreakVector` (`self.Forward`)))
  (bind _returnvalue (* (`self.TimeParsent`) (`self.BulletLenght`)))
  (bind (_returnvalue_x_2 _returnvalue_y_2 _returnvalue_z_2) (`KismetMathLibrary.BreakVector` (+ (`self.K2_GetActorLocation`) (* (`self.Forward`) 5.0))))
  (`parent.ReceiveTick` DeltaSeconds)
  (`self.UpdateTime` DeltaSeconds)
  (if (`self.TimeOut`)
    (if (<= _returnvalue_z 0.0)
      (`self.K2_DestroyActor`)
      (else
        (`self.K2_SetActorLocation` (`KismetMathLibrary.MakeVector` _returnvalue_x_2 _returnvalue_y_2 (- _returnvalue_z_2 15.0)))))
    (else
      (`self.K2_SetActorLocation` (`KismetMathLibrary.MakeVector` (+ (* _returnvalue _forward_x) _baseposition_x) (+ (* _returnvalue _forward_y) _baseposition_y) (+ (* (`KismetMathLibrary.DegSin` (* (`self.TimeParsent`) 180.0)) (`self.HeightLenght`)) _baseposition_z)))
      (`SceneComponent.K2_AddLocalRotation` (`self.Sphere`) (struct :`Pitch` 10.0) false false))))

(event `self.Sphere1.OnComponentBeginOverlap`
  (params (OverlappedComponent :type "PrimitiveComponent Object Reference") (OtherActor :type "Actor Object Reference") (OtherComp :type "PrimitiveComponent Object Reference") (OtherBodyIndex :type Integer) (bFromSweep :type Boolean) (SweepResult :type "HitResult Structure (by ref)"))
  (`/Engine/EditorBlueprintResources/StandardMacros.IsValid` (`self.FirePlayer`)
    (:`Is Valid`
      (bind _asbp_owner (cast `/Game/Character/BP_Owner` OtherActor))
      (if (!= _asbp_owner (`self.FirePlayer`))
        _))))

(fn `UserConstructionScript`
  (`parent.UserConstructionScript`))