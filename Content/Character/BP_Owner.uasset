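; Base player character handling movement, evasion, attacks, damage and death, with a status enum gating actions.
; Movement axes add world-space input and store a camera-yaw-relative stick direction, which evasion faces before a timeline-driven, frame-counted forward dash.
; Attack helpers set power, speed and rotation lock, damage other BP_Owner actors through a hit list meant to prevent repeats, and spawn bullets.
; Damage plays a montage; death launches the character randomly and disables collision.
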(event `self.ReceiveBeginPlay`
  (`self.Initialize`))

(event `self.ReceiveTick`
  (params (DeltaSeconds :type "Float (single-precision)")))

(event `InputAxis|MoveForWard`
  (params (AxisValue :type "Float (single-precision)"))
  ;[1 1 1] Move
  (if (`self.CanMove`)
    (`self.AddMovementInput` (1.0 0.0 0.0) AxisValue)
    (bind (_stickdown_ _stickdirection) (`self.GetLeftStickDown` AxisValue (stale `InputAxis|MoveRight` AxisValue) :!label _label))
    (bind _output_get (set `self.IsStickDown` _stickdown_))
    (if _output_get
      (set `self.LeftDirection` _stickdirection)
      (else
        (set `self.LeftDirection` (`self.GetActorForwardVector` self))))))

(event `InputAxis|MoveRight`
  (params (AxisValue :type "Float (single-precision)"))
  ;[1 1 1] Move
  (if (`self.CanMove`)
    (`self.AddMovementInput` (0.0 1.0 0.0) AxisValue)
    (goto _label)))

(event `self.ReceiveAnyDamage`
  (params (Damage :type "Float (single-precision)") (DamageType :type "DamageType Object Reference") (InstigatedBy :type "Controller Object Reference") (DamageCauser :type "Actor Object Reference"))
  ;[1 1 1] Damage
  (if (`|EnumInequality` (`self.PlayerStatus`) "NewEnumerator5")
    (`self.ReceiveDamage` Damage)))

(event `InputAction|Evasion`
  (params (Key :type "Key Structure"))
  ;[1 1 1] Evasion
  (:`Pressed`
    (`self.InitializeEvasion`)))

(event `EvasionStart`
  ;[1 1 1] Evasion
  (`Timeline|EvasionTick` :!via `PlayFromStart` :!label _label_2
    (:`Update`
      (`self.EvasionMove`))))

(event `EvasionEnd`
  ;[1 1 1] Evasion
  (goto _label_2 :!via `Stop`))

(event `DestroyPlayerMove`
  ;[1 1 1] Dead
  (`KismetSystemLibrary.Delay` 1.0)
  (`PrimitiveComponent.SetCollisionEnabled` (`self.Mesh`) "QueryAndPhysics")
  (`PrimitiveComponent.SetCollisionEnabled` (`self.CapsuleComponent`) "QueryAndPhysics")
  (set `MovementComponent.Velocity` (0.0 0.0 0.0) (`self.CharacterMovement`)))

(fn `AttackContinuou`
  (if (`self.IsAnimeLoop`)
    (set `self.IsAttackContinuou` true)))

(fn `AttackOption`
  (params (PlayerStatus :type "/Game/Character/PlayerStatus Enum" :default "NewEnumerator0") (AttackPower :type "Float (double-precision)") (MoveSpeed :type "Float (double-precision)") (DirectionFixed :type Boolean))
  (set `self.PlayerStatus` PlayerStatus)
  (`self.AttackSetting` AttackPower MoveSpeed)
  (set `self.IsAttackTiming` true)
  (set `self.KeyInputOK` false)
  (if DirectionFixed
    (`self.LongDistanceAttack`)))

(fn `AttackSetting`
  (params (AttackPower :type "Float (double-precision)") (MoveSpeed :type "Float (double-precision)"))
  (set `self.AttackPower` AttackPower)
  (set `CharacterMovementComponent.MaxWalkSpeed` MoveSpeed (`self.CharacterMovement`)))

(fn `BulletCreate`
  (params (SpawnLocation :type "Vector Structure"))
  (returns (ShotBullet :type "Actor Object Reference"))
  (bind _returnvalue (`|SpawnActorFromClass` (`self.MyBullet`) (`KismetMathLibrary.MakeTransform` SpawnLocation (`SceneComponent.K2_GetComponentRotation` (`self.CapsuleComponent`))) "Undefined" "OverrideRootScale" null null))
  (return _returnvalue))

(fn `CanAttack`
  (returns (KeyInputOK :type Boolean) (IsDash :type Boolean))
  (return (`self.KeyInputOK`) (> (`KismetMathLibrary.VSize` (`self.GetVelocity` self)) 0.0)))

(fn `CanMove`
  (returns (ReturnValue :type Boolean))
  (return (and (`|EnumInequality` (`self.PlayerStatus`) "NewEnumerator7") (`self.IsGame`))))

(fn `EvasionMove`
  (if (>= (`self.EvasionFlameCount`) 0)
    (`self.K2_AddActorLocalOffset` (`KismetMathLibrary.MakeVector` (`self.EvasionSpeed`)))
    (`/Engine/EditorBlueprintResources/StandardMacros.DecrementInt` (`self.EvasionFlameCount`))
    (else
      (set `self.PlayerStatus` "NewEnumerator0")
      (`self.EvasionEnd`))))

(fn `GetLeftStickDown`
  (params (Xinput :type "Float (double-precision)") (Yinput :type "Float (double-precision)"))
  (returns (`StickDown?` :type Boolean) (StickDirection :type "Vector Structure"))
  (bind _returnvalue (`KismetMathLibrary.MakeRotator` 0.0 0.0 (.yaw (`self.GetControlRotation`))))
  (bind _returnvalue_2 (+ (* (`KismetMathLibrary.GetForwardVector` _returnvalue) Xinput) (* (`KismetMathLibrary.GetRightVector` _returnvalue) Yinput)))
  (return (>= (`KismetMathLibrary.VSize` _returnvalue_2) 0.5) _returnvalue_2))

(fn `HitActorDuplication`
  (params (Object :type "Object Object Reference"))
  (bind _asbp_owner (cast `/Game/Character/BP_Owner` Object))
  (set `self.HitActor` _asbp_owner)
  (for _array_element (`self.AttackHitActor`)
    ;[1 1 1] 今HitしているActorが初めてHitした場合フラグを立てる
    (set `self.AttackHit` (== _array_element (`self.HitActor`))))
  (if (and (!= _asbp_owner self) (not (`self.AttackHit`)))
    (`self.SendDamage` (`self.HitActor`) (`self.AttackPower`))
    (`KismetArrayLibrary.Array_Add` (`self.AttackHitActor`) (`self.HitActor`))))

(fn `Initialize`
  (set `self.Life` (`self.DefaultLife`)))

(fn `InitializeEvasion`
  (if (`|EnumEquality` (`self.PlayerStatus`) "NewEnumerator0")
    (set `self.PlayerStatus` "NewEnumerator8")
    (`self.K2_SetActorRotation` (`KismetMathLibrary.Conv_VectorToRotator` (`self.LeftDirection`)))
    (set `self.EvasionFlameCount` (`self.DefaultEvasionFlame`))
    (`self.EvasionStart`)))

(fn `LongDistanceAttack`
  (set `CharacterMovementComponent.bOrientRotationToMovement` false (`self.CharacterMovement`)))

(fn `PlayerDead`
  (set `self.PlayerStatus` "NewEnumerator7")
  ;[1 1 1] 吹き飛ばし
  (`self.LaunchCharacter` (`KismetMathLibrary.MakeVector` (`KismetMathLibrary.RandomFloatInRange` -10000.0 10000.0) (`KismetMathLibrary.RandomFloatInRange` -10000.0 10000.0) 200.0))
  (`PrimitiveComponent.SetCollisionEnabled` (`self.Mesh`) "NoCollision")
  (`PrimitiveComponent.SetCollisionEnabled` (`self.CapsuleComponent`) "NoCollision")
  (set `self.IsGame` false))

(fn `ReceiveDamage`
  (params (Damage :type "Float (double-precision)"))
  (bind _output_get (set `self.Life` (- (`self.Life`) Damage)))
  (if (<= _output_get 0.0)
    (`self.PlayerDead`)
    (else
      (set `self.PlayerStatus` "NewEnumerator5")
      (`self.PlayAnimMontage` "/Game/Character/MID-3/Anime/Damage.Damage"))))

(fn `SendDamage`
  (params (DamagedActor :type "Actor Object Reference") (BaseDamage :type "Float (double-precision)"))
  (`GameplayStatics.ApplyDamage` DamagedActor BaseDamage))

(fn `UserConstructionScript`)