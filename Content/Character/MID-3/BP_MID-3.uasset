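; MID-3 character Blueprint with four attacks: electric shot, missile, grenade and a Chariot laser special.
; Each input passes the parent's attack checks, sets state and movement options through AttackOption, and selects the bullet.
; The special also starts the Laser beam animation, with a separate function for ending it.
; BoosterSet attaches four booster emitters; Tick toggles movement and evasion pairs from movement and PlayerStatus, using cross-resetting DoOnce nodes.
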(event `self.ReceiveBeginPlay`
  (`parent.ReceiveBeginPlay`)
  (`self.BoosterSet`)
  (`self.InitializeStatus` "MID-3"))

(event `self.ReceiveTick`
  (params (DeltaSeconds :type "Float (single-precision)"))
  (`parent.ReceiveTick` DeltaSeconds)
  (`self.CreateBooster`))

(event `InputAction|FirstAttack`
  (params (Key :type "Key Structure"))
  (bind _mybullets_firstattack (break `/Game/Weapons/resource/S_Weapons` (`self.MyBullets`)))
  ;[1 1 1] Attack
  (:`Pressed`
    (`self.AttackContinuou`)
    (if (`self.CanAttack`)
      (`self.AttackOption` "NewEnumerator1" 0.0 600.0 true true)
      (set `self.MyBullet` _mybullets_firstattack))))

(event `InputAction|SecondAttack`
  (params (Key :type "Key Structure"))
  (bind (_mybullets_firstattack _mybullets_secondattack) (break `/Game/Weapons/resource/S_Weapons` (`self.MyBullets`)))
  ;[1 1 1] Attack
  (:`Pressed`
    (if (`self.CanAttack`)
      (`self.AttackOption` "NewEnumerator2" 0.0 600.0 false true)
      (set `self.MyBullet` _mybullets_secondattack))))

(event `InputAction|UniqueAttack`
  (params (Key :type "Key Structure"))
  (bind (_mybullets_firstattack _mybullets_secondattack _mybullets_uniqueattack) (break `/Game/Weapons/resource/S_Weapons` (`self.MyBullets`)))
  ;[1 1 1] Attack
  (:`Pressed`
    (if (`self.CanAttack`)
      (`self.AttackOption` "NewEnumerator3" 0.0 0.0 false true)
      (set `self.MyBullet` _mybullets_uniqueattack))))

(event `InputAction|SpecialAttack`
  (params (Key :type "Key Structure"))
  (bind (_mybullets_firstattack _mybullets_secondattack _mybullets_uniqueattack _mybullets_specialattack) (break `/Game/Weapons/resource/S_Weapons` (`self.MyBullets`)))
  ;[1 1 1] Attack
  (:`Pressed`
    (if (and (`self.CanAttack`) (`self.CanSpecialAttack`))
      (`self.AttackOption` "NewEnumerator4" 0.0 0.0 false true)
      (set `self.MyBullet` _mybullets_specialattack)
      (`self.LaserBeamStart`))))

(fn `BoosterSet`
  (bind _returnvalue (`GameplayStatics.SpawnEmitterAttached` "/Game/Effect/Booster/Particle/P_Booster.P_Booster" (`self.Mesh`) "Booster_1"))
  (bind _returnvalue_2 (`GameplayStatics.SpawnEmitterAttached` "/Game/Effect/Booster/Particle/P_Booster.P_Booster" (`self.Mesh`) "Booster_2"))
  (set `self.MoveBoosters` (`|MakeArray` _returnvalue _returnvalue_2))
  (bind _returnvalue_3 (`GameplayStatics.SpawnEmitterAttached` "/Game/Effect/Booster/Particle/P_Booster.P_Booster" (`self.Mesh`) "Booster_3"))
  (bind _returnvalue_4 (`GameplayStatics.SpawnEmitterAttached` "/Game/Effect/Booster/Particle/P_Booster.P_Booster" (`self.Mesh`) "Booster_4"))
  (set `self.EvasionBoosters` (`|MakeArray` _returnvalue_3 _returnvalue_4)))

(fn `CreateBooster`
  (bind _moveboosters (`self.MoveBoosters`))
  (bind _evasionboosters (`self.EvasionBoosters`))
  (`|ExecutionSequence`
    (:`then_0`
      (if (and (`self.IsStickDown`) (>= (`KismetMathLibrary.VSize` (`self.GetVelocity` self)) 2.0))
        (`/Engine/EditorBlueprintResources/StandardMacros.DoOnce` false :!label _label
          (:`Completed`
            (for _array_element _moveboosters
              (`SceneComponent.SetVisibility` _array_element true false)
              (goto _label_2 :!via `Reset`))))
        (else
          (`/Engine/EditorBlueprintResources/StandardMacros.DoOnce` false :!label _label_2
            (:`Completed`
              (for _array_element_2 _moveboosters
                (`SceneComponent.SetVisibility` _array_element_2 false false)
                (goto _label :!via `Reset`)))))))
    (:`then_1`
      (if (`|EnumEquality` (`self.PlayerStatus`) "NewEnumerator8")
        (`/Engine/EditorBlueprintResources/StandardMacros.DoOnce` false :!label _label_3
          (:`Completed`
            (for _array_element_3 _evasionboosters
              (`SceneComponent.SetVisibility` _array_element_3 true false)
              (goto _label_4 :!via `Reset`))))
        (else
          (`/Engine/EditorBlueprintResources/StandardMacros.DoOnce` false :!label _label_4
            (:`Completed`
              (for _array_element_4 _evasionboosters
                (`SceneComponent.SetVisibility` _array_element_4 false false)
                (goto _label_3 :!via `Reset`)))))))))

(fn `LaserBeamEnd`
  (`SkeletalMeshComponent.PlayAnimation` (`self.Laser`) "/Game/Weapons/MID-3/Laser/LaserBeam/Chariot_LaserBeamOver.Chariot_LaserBeamOver" false))

(fn `LaserBeamStart`
  (bind _laser (`self.Laser`))
  (`SceneComponent.SetVisibility` _laser true false)
  (`SkeletalMeshComponent.PlayAnimation` _laser "/Game/Weapons/MID-3/Laser/LaserBeam/Chariot_LaserBeam.Chariot_LaserBeam" false))

(fn `UserConstructionScript`
  (`parent.UserConstructionScript`))