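; Lou's player character Blueprint, implementing a cleaning-themed moveset on top of its parent class: broom, dash mop, bucket swing, hairball throw and dust-cloth special.
; Inputs pass parent attack checks, then set PlayerStatus, which WeaponCreate uses to reveal a preplaced child-actor weapon.
; Separate events toggle that weapon's hitbox.
; Timelines drive swept movement: dash runs while in FirstAttack, special counts down frames before returning to Idle.
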(event `self.ReceiveBeginPlay`
  (`parent.ReceiveBeginPlay`)
  (`self.InitializeStatus` "Lou")
  (`self.InitWeapon`))

(event `self.ReceiveTick`
  (params (DeltaSeconds :type "Float (single-precision)"))
  (`parent.ReceiveTick` DeltaSeconds))

(event `WeaponCollisionON`
  (bind _attackweapon (`self.AttackWeapon`))
  ;[1 1 1] 武器の当たり判定ONOFF
  (`/Engine/EditorBlueprintResources/StandardMacros.IsValid` _attackweapon
    (:`Is Valid`
      (bind _asbp_proximity_weapons (cast `/Game/Weapons/resource/BP_ProximityWeapons` (`ChildActorComponent.ChildActor` _attackweapon)))
      (`/Game/Weapons/resource/BP_ProximityWeapons.AttackON` _asbp_proximity_weapons))))

(event `InputAction|FirstAttack`
  (params (Key :type "Key Structure"))
  (bind (_keyinputok _isdash) (`self.CanAttack`))
  ;[1 1 1] Attack
  (:`Pressed`
    (if _keyinputok
      (if _isdash
        (`self.AttackOption` "NewEnumerator1")
        (set `self.IsDashAttack` true)
        (`self.WeaponCreate`)
        (`self.DashAttackStart`)
        (else
          (`self.AttackOption` "NewEnumerator1" 0.0 0.0 false true)
          (`self.WeaponCreate`))))))

(event `SpecialAttackStart`
  ;[1 1 1] 雑巾がけ
  (`Timeline|SpecialAttackTick` :!via `PlayFromStart` :!label _label
    (:`Update`
      (`self.SpecialAttackMove`))))

(event `SpecialAttackEnd`
  ;[1 1 1] 雑巾がけ
  (goto _label :!via `Stop`))

(event `WeaponCollisionOFF`
  (bind _attackweapon (`self.AttackWeapon`))
  ;[1 1 1] 武器の当たり判定ONOFF
  (`/Engine/EditorBlueprintResources/StandardMacros.IsValid` _attackweapon
    (:`Is Valid`
      (bind _asbp_proximity_weapons (cast `/Game/Weapons/resource/BP_ProximityWeapons` (`ChildActorComponent.ChildActor` _attackweapon)))
      (`/Game/Weapons/resource/BP_ProximityWeapons.AttackOFF` _asbp_proximity_weapons))))

(event `DashAttackStart`
  ;[1 1 1] モップがけ
  (`Timeline|DashAttackTick` :!via `PlayFromStart` :!label _label_2
    (:`Update`
      (`self.DashAttackMove`))))

(event `InputAction|SecondAttack`
  (params (Key :type "Key Structure"))
  ;[1 1 1] Attack
  (:`Pressed`
    (if (`self.CanAttack`)
      (`self.AttackOption` "NewEnumerator2" 0.0 200.0 false true)
      (`self.WeaponCreate`))))

(event `DashAttackEnd`
  ;[1 1 1] モップがけ
  (goto _label_2 :!via `Stop`))

(event `InputAction|UniqueAttack`
  (params (Key :type "Key Structure"))
  (bind (_mybullets_firstattack _mybullets_secondattack _mybullets_uniqueattack) (break `/Game/Weapons/resource/S_Weapons` (`self.MyBullets`)))
  ;[1 1 1] Attack
  (:`Pressed`
    (if (`self.CanAttack`)
      (`self.AttackOption` "NewEnumerator3" 0.0 0.0 false true)
      (set `self.MyBullet` _mybullets_uniqueattack))))

(event `InputAction|SpecialAttack`
  (params (Key :type "Key Structure"))
  ;[1 1 1] Attack
  (:`Pressed`
    (if (and (`self.CanAttack`) (`self.CanSpecialAttack`))
      (`self.AttackOption` "NewEnumerator4")
      (`self.WeaponCreate`))))

(fn `DashAttackMove`
  (locals (DASpeed :type "Float (double-precision)" :default 5.0))
  (if (`|EnumEquality` (`self.PlayerStatus`) "NewEnumerator1")
    (`self.K2_AddActorWorldOffset` (* (`self.GetActorForwardVector` self) (`local.DASpeed`)) true)
    (else
      (`self.DashAttackEnd`))))

(fn `InitializeSpecialAttack`
  (set `self.SAFlameCount` (`self.DefaultSAFlameCount`))
  (`self.SpecialAttackStart`))

(fn `InitWeapon`
  (for _array_element (`|MakeArray` (`self.BP_Broom`) (`self.BP_DustCloth`) (`self.BP_Bucket`) (`self.BP_Mop`))
    (bind _asbp_proximity_weapons (cast `/Game/Weapons/resource/BP_ProximityWeapons` (`ChildActorComponent.ChildActor` _array_element)))
    (set `/Game/Weapons/resource/BP_ProximityWeapons.MyOwner` self _asbp_proximity_weapons)))

(fn `SpecialAttackMove`
  (if (>= (`self.SAFlameCount`) 0)
    (`self.K2_AddActorWorldOffset` (* (`self.LeftDirection`) (`self.SASpeed`)) true)
    (`/Engine/EditorBlueprintResources/StandardMacros.DecrementInt` (`self.SAFlameCount`))
    (else
      (set `self.PlayerStatus` "NewEnumerator0")
      (`self.SpecialAttackEnd`))))

(fn `UserConstructionScript`
  (`parent.UserConstructionScript`))

(fn `WeaponCreate`
  (switch `/Game/Character/PlayerStatus` (`self.PlayerStatus`)
    (:`NewEnumerator1`
      (if (`.IsDash` (`self.CanAttack`))
        (bind _output_get (set `self.AttackWeapon` (`self.BP_Mop`)))
        (`SceneComponent.SetVisibility` _output_get true false)
        (else
          (bind _output_get_2 (set `self.AttackWeapon` (`self.BP_Broom`)))
          (`SceneComponent.SetVisibility` _output_get_2 true false)
          (`SceneComponent.SetVisibility` (`self.lou_weapon_broom`) false false))))
    (:`NewEnumerator2`
      (bind _output_get_3 (set `self.AttackWeapon` (`self.BP_Bucket`)))
      (`SceneComponent.SetVisibility` _output_get_3 true false))
    (:`NewEnumerator4`
      (bind _output_get_4 (set `self.AttackWeapon` (`self.BP_DustCloth`)))
      (`SceneComponent.SetVisibility` _output_get_4 true false))))

(fn `WeaponRemove`
  (bind _attackweapon (`self.AttackWeapon`))
  (`/Engine/EditorBlueprintResources/StandardMacros.IsValid` _attackweapon
    (:`Is Valid`
      (`SceneComponent.SetVisibility` _attackweapon false false)
      (if (not (`SceneComponent.bVisible` (`self.lou_weapon_broom`)))
        (`SceneComponent.SetVisibility` (`self.lou_weapon_broom`) true false)))))