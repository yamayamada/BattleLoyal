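; Playable character Iris, with four input-driven attacks: vertical slash, spinning slash, machete throw and a felling special.
; Each input passes CanAttack, plus CanSpecialAttack for the special, then sets state through AttackOption; the throw also selects a bullet type.
; Tick runs AttackCollision, which uses paired DoOnce gates to switch the hit Box with the two slash states.
; Box overlaps send AttackPower damage to other BP_Owner actors.
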(event `self.ReceiveBeginPlay`
  (`parent.ReceiveBeginPlay`)
  (`self.InitializeStatus` "Iris"))

(event `self.ReceiveTick`
  (params (DeltaSeconds :type "Float (single-precision)"))
  (`parent.ReceiveTick` DeltaSeconds)
  (`self.AttackCollision`))

(event `InputAction|FirstAttack`
  (params (Key :type "Key Structure"))
  ;[1 1 1] Attack
  (:`Pressed`
    (if (`self.CanAttack`)
      (`self.AttackOption` "NewEnumerator1" 20.0 0.0 false true))))

(event `InputAction|SecondAttack`
  (params (Key :type "Key Structure"))
  ;[1 1 1] Attack
  (:`Pressed`
    (if (`self.CanAttack`)
      (`self.AttackOption` "NewEnumerator2" 20.0 0.0 false true))))

(event `InputAction|UniqueAttack`
  (params (Key :type "Key Structure"))
  (bind (_mybullets_firstattack _mybullets_secondattack _mybullets_uniqueattack) (break `/Game/Weapons/resource/S_Weapons` (`self.MyBullets`)))
  ;[1 1 1] Attack
  (:`Pressed`
    (if (`self.CanAttack`)
      (`self.AttackOption` "NewEnumerator3" 0.0 0.0 false true)
      (set `self.MyBullet` _mybullets_uniqueattack))))

(event `InputAction|SpecialAttack`
  (params (Key :type "Key Structure"))
  ;[1 1 1] Attack
  (:`Pressed`
    (if (and (`self.CanAttack`) (`self.CanSpecialAttack`))
      (`self.AttackOption` "NewEnumerator4" 0.0 0.0 false true))))

(event `self.Box.OnComponentBeginOverlap`
  (params (OverlappedComponent :type "PrimitiveComponent Object Reference") (OtherActor :type "Actor Object Reference") (OtherComp :type "PrimitiveComponent Object Reference") (OtherBodyIndex :type Integer) (bFromSweep :type Boolean) (SweepResult :type "HitResult Structure (by ref)"))
  (bind _asbp_owner (cast `/Game/Character/BP_Owner` OtherActor))
  (if (!= _asbp_owner self)
    (`self.SendDamage` self _asbp_owner (`self.AttackPower`))))

(fn `AttackCollision`
  (bind _playerstatus (`self.PlayerStatus`))
  (bind _box (`self.Box`))
  (if (or (`|EnumEquality` _playerstatus "NewEnumerator1") (`|EnumEquality` _playerstatus "NewEnumerator2"))
    (`/Engine/EditorBlueprintResources/StandardMacros.DoOnce` false :!label _label
      (:`Completed`
        (`PrimitiveComponent.SetCollisionEnabled` _box "QueryAndPhysics")
        (goto _label_2 :!via `Reset`)))
    (else
      (`/Engine/EditorBlueprintResources/StandardMacros.DoOnce` false :!label _label_2
        (:`Completed`
          (`PrimitiveComponent.SetCollisionEnabled` _box "NoCollision")
          (goto _label :!via `Reset`))))))

(fn `UserConstructionScript`
  (`parent.UserConstructionScript`))