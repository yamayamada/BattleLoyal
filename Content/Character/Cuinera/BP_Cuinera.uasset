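; BP_Cuinera is the playable cook character Cuinera, built on a parent character Blueprint and initialized with the CookCuinera status.
; Attack inputs gated by CanAttack set an attack state with fixed facing: tableware throw, frying-pan boomerang, counter, and a special that also requires CanSpecialAttack.
; The two projectile attacks select their bullet from MyBullets.
; Holding the counter input shows the Chinese hotpot weapon with physics-only collision; releasing hides it and resets the state.
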(event `self.ReceiveBeginPlay`
  (`parent.ReceiveBeginPlay`)
  (`self.InitializeStatus` "CookCuinera"))

(event `self.ReceiveTick`
  (params (DeltaSeconds :type "Float (single-precision)"))
  (`parent.ReceiveTick` DeltaSeconds))

(event `InputAction|FirstAttack`
  (params (Key :type "Key Structure"))
  (bind _mybullets_firstattack (break `/Game/Weapons/resource/S_Weapons` (`self.MyBullets`)))
  ;[1 1 1] Attack
  (:`Pressed`
    (if (`self.CanAttack`)
      (`self.AttackOption` "NewEnumerator1" 0.0 0.0 false true)
      (set `self.MyBullet` _mybullets_firstattack))))

(event `InputAction|SecondAttack`
  (params (Key :type "Key Structure"))
  (bind (_mybullets_firstattack _mybullets_secondattack) (break `/Game/Weapons/resource/S_Weapons` (`self.MyBullets`)))
  ;[1 1 1] Attack
  (:`Pressed`
    (if (`self.CanAttack`)
      (`self.AttackOption` "NewEnumerator2" 0.0 0.0 false true)
      (set `self.MyBullet` _mybullets_secondattack))))

(event `InputAction|UniqueAttack`
  (params (Key :type "Key Structure"))
  ;[1 1 1] Attack
  (:`Pressed`
    (if (`self.CanAttack`)
      (`self.AttackOption` "NewEnumerator3" 0.0 0.0 false true)
      (`self.CounterSet` true)))
  (:`Released`
    (`self.CounterSet` false)))

(event `InputAction|SpecialAttack`
  (params (Key :type "Key Structure"))
  ;[1 1 1] Attack
  (:`Pressed`
    (if (and (`self.CanAttack`) (`self.CanSpecialAttack`))
      (`self.AttackOption` "NewEnumerator4" 0.0 0.0 false true))))

(fn `CounterSet`
  (params (IsCounter :type Boolean))
  (bind _cook_weapon__chinesehotpot (`self.cook_weapon__Chinesehotpot`))
  (bind _cook_weapon__chinesehotpot_2 (`self.cook_weapon__Chinesehotpot`))
  (if IsCounter
    (set `self.IsCounter` true)
    (`SceneComponent.SetVisibility` _cook_weapon__chinesehotpot_2 true false)
    (`PrimitiveComponent.SetCollisionEnabled` _cook_weapon__chinesehotpot_2 "PhysicsOnly")
    (else
      (set `self.IsCounter` false)
      (set `self.PlayerStatus` "NewEnumerator0")
      (`SceneComponent.SetVisibility` _cook_weapon__chinesehotpot false false)
      (`PrimitiveComponent.SetCollisionEnabled` _cook_weapon__chinesehotpot "NoCollision"))))

(fn `UserConstructionScript`
  (`parent.UserConstructionScript`))