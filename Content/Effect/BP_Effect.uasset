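; BP_Effect is an effect Blueprint that plays a looping flipbook animation on a supplied material by stepping through a sprite-sheet grid.
; Init stores the material, speed, grid size and frame count, passes the grid size to the material, then starts the Animation event.
; Animation converts Count into column and row UV offsets, wraps it at Frames, and re-calls itself after a Delay instead of using Tick.
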(event `self.ReceiveBeginPlay`)

(event `Animation`
  (bind _wight (`self.Wight`))
  (bind _count (`self.Count`))
  (`MaterialInstanceDynamic.SetScalarParameterValue` (`self.material`) "U_Tiling" (* (mod _count _wight) (/ 1.0 (`KismetMathLibrary.Conv_IntToDouble` _wight))))
  (`MaterialInstanceDynamic.SetScalarParameterValue` (`self.material`) "V_Tiling" (* (/ _count _wight) (/ 1.0 (`KismetMathLibrary.Conv_IntToDouble` (`self.Height`)))))
  (bind _result (`/Engine/EditorBlueprintResources/StandardMacros.IncrementInt` (`self.Count`))
    (:`  `
      (if (>= _result (`self.Frames`))
        (set `self.Count` 0))
      (`KismetSystemLibrary.Delay` (`self.AnimationSpeed`))
      (`self.Animation`))))

(fn `Init`
  (params (material :type "MaterialInstanceDynamic Object Reference") (AnimationSpeed :type "Float (double-precision)") (Wight :type Integer) (Height :type Integer) (Frames :type Integer))
  (set `self.material` material)
  (set `self.AnimationSpeed` AnimationSpeed)
  (set `self.Wight` Wight)
  (set `self.Height` Height)
  (set `self.Frames` Frames)
  (`MaterialInstanceDynamic.SetScalarParameterValue` (`self.material`) "Wight" (`KismetMathLibrary.Conv_IntToDouble` (`self.Wight`)))
  (`MaterialInstanceDynamic.SetScalarParameterValue` (`self.material`) "Height" (`KismetMathLibrary.Conv_IntToDouble` (`self.Height`)))
  (`self.Animation`))

(fn `UserConstructionScript`)