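; BP_CounterFire is a short-lived fire effect actor that deals counter damage to BP_Owner actors that touch it.
; Eight capsule components each handle begin overlap, casting the other actor to BP_Owner and calling its SendDamage with CounterDamage.
; Each capsule triggers independently, so one target can be hit by several capsules.
; Tick counts LifeTimer down and destroys the actor when it runs out.
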(event `self.ReceiveTick`
  (params (DeltaSeconds :type "Float (single-precision)"))
  (bind _output_get (set `self.LifeTimer` (- (`self.LifeTimer`) DeltaSeconds)))
  (if (<= _output_get 0.0)
    (`self.K2_DestroyActor`)))

(event `self.Capsule.OnComponentBeginOverlap`
  (params (OverlappedComponent :type "PrimitiveComponent Object Reference") (OtherActor :type "Actor Object Reference") (OtherComp :type "PrimitiveComponent Object Reference") (OtherBodyIndex :type Integer) (bFromSweep :type Boolean) (SweepResult :type "HitResult Structure (by ref)"))
  (bind _asbp_owner (cast `/Game/Character/BP_Owner` OtherActor))
  (`/Game/Character/BP_Owner.SendDamage` _asbp_owner _asbp_owner (`self.CounterDamage`)))

(event `self.Capsule1.OnComponentBeginOverlap`
  (params (OverlappedComponent :type "PrimitiveComponent Object Reference") (OtherActor :type "Actor Object Reference") (OtherComp :type "PrimitiveComponent Object Reference") (OtherBodyIndex :type Integer) (bFromSweep :type Boolean) (SweepResult :type "HitResult Structure (by ref)"))
  (bind _asbp_owner (cast `/Game/Character/BP_Owner` OtherActor))
  (`/Game/Character/BP_Owner.SendDamage` _asbp_owner _asbp_owner (`self.CounterDamage`)))

(event `self.Capsule2.OnComponentBeginOverlap`
  (params (OverlappedComponent :type "PrimitiveComponent Object Reference") (OtherActor :type "Actor Object Reference") (OtherComp :type "PrimitiveComponent Object Reference") (OtherBodyIndex :type Integer) (bFromSweep :type Boolean) (SweepResult :type "HitResult Structure (by ref)"))
  (bind _asbp_owner (cast `/Game/Character/BP_Owner` OtherActor))
  (`/Game/Character/BP_Owner.SendDamage` _asbp_owner _asbp_owner (`self.CounterDamage`)))

(event `self.Capsule3.OnComponentBeginOverlap`
  (params (OverlappedComponent :type "PrimitiveComponent Object Reference") (OtherActor :type "Actor Object Reference") (OtherComp :type "PrimitiveComponent Object Reference") (OtherBodyIndex :type Integer) (bFromSweep :type Boolean) (SweepResult :type "HitResult Structure (by ref)"))
  (bind _asbp_owner (cast `/Game/Character/BP_Owner` OtherActor))
  (`/Game/Character/BP_Owner.SendDamage` _asbp_owner _asbp_owner (`self.CounterDamage`)))

(event `self.Capsule4.OnComponentBeginOverlap`
  (params (OverlappedComponent :type "PrimitiveComponent Object Reference") (OtherActor :type "Actor Object Reference") (OtherComp :type "PrimitiveComponent Object Reference") (OtherBodyIndex :type Integer) (bFromSweep :type Boolean) (SweepResult :type "HitResult Structure (by ref)"))
  (bind _asbp_owner (cast `/Game/Character/BP_Owner` OtherActor))
  (`/Game/Character/BP_Owner.SendDamage` _asbp_owner _asbp_owner (`self.CounterDamage`)))

(event `self.Capsule5.OnComponentBeginOverlap`
  (params (OverlappedComponent :type "PrimitiveComponent Object Reference") (OtherActor :type "Actor Object Reference") (OtherComp :type "PrimitiveComponent Object Reference") (OtherBodyIndex :type Integer) (bFromSweep :type Boolean) (SweepResult :type "HitResult Structure (by ref)"))
  (bind _asbp_owner (cast `/Game/Character/BP_Owner` OtherActor))
  (`/Game/Character/BP_Owner.SendDamage` _asbp_owner _asbp_owner (`self.CounterDamage`)))

(event `self.Capsule6.OnComponentBeginOverlap`
  (params (OverlappedComponent :type "PrimitiveComponent Object Reference") (OtherActor :type "Actor Object Reference") (OtherComp :type "PrimitiveComponent Object Reference") (OtherBodyIndex :type Integer) (bFromSweep :type Boolean) (SweepResult :type "HitResult Structure (by ref)"))
  (bind _asbp_owner (cast `/Game/Character/BP_Owner` OtherActor))
  (`/Game/Character/BP_Owner.SendDamage` _asbp_owner _asbp_owner (`self.CounterDamage`)))

(event `self.Capsule7.OnComponentBeginOverlap`
  (params (OverlappedComponent :type "PrimitiveComponent Object Reference") (OtherActor :type "Actor Object Reference") (OtherComp :type "PrimitiveComponent Object Reference") (OtherBodyIndex :type Integer) (bFromSweep :type Boolean) (SweepResult :type "HitResult Structure (by ref)"))
  (bind _asbp_owner (cast `/Game/Character/BP_Owner` OtherActor))
  (`/Game/Character/BP_Owner.SendDamage` _asbp_owner _asbp_owner (`self.CounterDamage`)))

(fn `UserConstructionScript`)