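; BP_Fire is a fire effect actor, apparently an animated flipbook drawn on its Plate component.
; On BeginPlay, it creates a dynamic instance of the Plate's first material and passes it to Init with animation speed, dimensions and frame count from Status.
; The Init logic is defined outside this graph; Tick, overlap and construction add no behavior of their own.
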(event `self.ReceiveBeginPlay`
  (bind (_status_animationspeed _status_wight _status_height _status_frames) (break `/Game/Effect/S_EffectStatus` (`self.Status`)))
  (`parent.ReceiveBeginPlay`)
  (bind _returnvalue (`PrimitiveComponent.CreateDynamicMaterialInstance` (`self.Plate`) 0 (`PrimitiveComponent.GetMaterial` (`self.Plate`) 0) "None"))
  (`self.Init` _returnvalue _status_animationspeed _status_wight _status_height _status_frames))

(fn `UserConstructionScript`
  (`parent.UserConstructionScript`))