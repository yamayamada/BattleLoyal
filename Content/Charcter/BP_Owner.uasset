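; BP_Owner is a player-controlled character Blueprint that handles movement and attack input.
; The MoveForWard and MoveRight axes feed AddMovementInput along fixed world X and Y, so movement ignores camera and actor rotation.
; The First, Second, Unique and Special attack presses each only set PlayerStatus to a different enum value, with no attack logic or status reset in these graphs.
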(event `InputAxis|MoveForWard`
  (params (AxisValue :type "Float (single-precision)"))
  ;[1 1 1] Move
  (`self.AddMovementInput` (1.0 0.0 0.0) AxisValue))

(event `InputAxis|MoveRight`
  (params (AxisValue :type "Float (single-precision)"))
  ;[1 1 1] Move
  (`self.AddMovementInput` (0.0 1.0 0.0) AxisValue))

(event `InputAction|FirstAttack`
  (params (Key :type "Key Structure"))
  (:`Pressed`
    (set `self.PlayerStatus` "NewEnumerator1")))

(event `InputAction|SecondAttack`
  (params (Key :type "Key Structure"))
  (:`Pressed`
    (set `self.PlayerStatus` "NewEnumerator2")))

(event `InputAction|UniqueAttack`
  (params (Key :type "Key Structure"))
  (:`Pressed`
    (set `self.PlayerStatus` "NewEnumerator3")))

(event `InputAction|SpecialAttack`
  (params (Key :type "Key Structure"))
  (:`Pressed`
    (set `self.PlayerStatus` "NewEnumerator4")))

(fn `UserConstructionScript`)